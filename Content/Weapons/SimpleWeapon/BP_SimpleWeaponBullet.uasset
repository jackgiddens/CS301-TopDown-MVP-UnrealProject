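; BP_SimpleWeaponBullet is the bullet for the simple gun, damaging actors that implement the EnemyDetection interface when they overlap its sphere.
; On overlap it loops over every BP_SimpleGunWeapon in the level, applying that weapon's BulletDamage scaled by a tenth of the player's temporary Damage stat.
; DestroyActor runs inside that loop after each damage call.
; CritChance and CritDamage lookups exist but are unused.
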(event `self.Sphere.OnComponentBeginOverlap`
  (params (OverlappedComponent :type "PrimitiveComponent Object Reference") (OtherActor :type "Actor Object Reference") (OtherComp :type "PrimitiveComponent Object Reference") (OtherBodyIndex :type Integer) (bFromSweep :type Boolean) (SweepResult :type "HitResult Structure (by ref)"))
  (if (`KismetSystemLibrary.DoesImplementInterface` OtherActor "/Game/Interfaces/EnemyDetection.EnemyDetection_C")
    (bind _outactors (`GameplayStatics.GetAllActorsOfClass` "/Game/Weapons/SimpleWeapon/BP_SimpleGunWeapon.BP_SimpleGunWeapon_C"))
    (for _array_element _outactors
      (bind _asbp_simple_gun_weapon (cast `/Game/Weapons/SimpleWeapon/BP_SimpleGunWeapon` _array_element))
      (bind _asbp_third_person_character (cast `/Game/ThirdPerson/Blueprints/BP_ThirdPersonCharacter` (`GameplayStatics.GetPlayerCharacter` 0)))
      (`GameplayStatics.ApplyDamage` OtherActor (* (`/Game/Weapons/SimpleWeapon/BP_SimpleGunWeapon.BulletDamage` _asbp_simple_gun_weapon) (* (`KismetMathLibrary.Conv_IntToDouble` (`BlueprintMapLibrary.Map_Find` (`/Game/ThirdPerson/Blueprints/BP_ThirdPersonCharacter.TempPlayerStats` _asbp_third_person_character) "Damage")) 0.1)) (`GameplayStatics.GetPlayerController` 0) _asbp_simple_gun_weapon)
      (`self.K2_DestroyActor`))))

(fn `UserConstructionScript`)