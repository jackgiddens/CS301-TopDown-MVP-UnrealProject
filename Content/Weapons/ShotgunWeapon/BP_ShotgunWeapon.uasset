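; Auto-firing shotgun that attaches to the player and shoots the nearest enemy without input.
; Tick picks the closest EnemyDetection actor from a range-sized sphere, then fires if it is in range with clear line of sight, using Delay as the fire-rate gate.
; Each shot spawns a yaw fan of shell actors with random cone jitter, passing damage and range.
; An empty magazine triggers a reload shortened by the player's ReloadSpeed stat.
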(event `FireWeapon`
  (bind _arrow (`self.Arrow`))
  (`/Engine/EditorBlueprintResources/StandardMacros.IsValid` (`self.ClosestEnemy`)
    (:`Is Valid`
      (bind (_outhit _returnvalue) (`KismetSystemLibrary.LineTraceSingle` (`self.K2_GetActorLocation` (`GameplayStatics.GetPlayerCharacter` 0)) (`self.K2_GetActorLocation` (`self.ClosestEnemy`)) "TraceTypeQuery1"))
      (if _returnvalue
        _
        (elif (< (`KismetMathLibrary.VSize` (- (`self.K2_GetActorLocation` (`GameplayStatics.GetPlayerCharacter` 0)) (`self.K2_GetActorLocation` (`self.ClosestEnemy`)))) (`self.Range`))
          (`SceneComponent.K2_SetWorldRotation` (`self.Arrow`) (`KismetMathLibrary.FindLookAtRotation` (`self.K2_GetActorLocation`) (`self.K2_GetActorLocation` (`self.ClosestEnemy`))) false false)
          (`KismetSystemLibrary.Delay` (`self.FireRate`))
          (set `self.Ammo` (- (`self.Ammo`) 1.0))
          (set `self.CurrentYaw` (`self.SpreadMax`))
          (for _ (range (+ (`KismetMathLibrary.FTrunc` (- (* (/ (`self.SpreadMax`) (`self.SpreadIncrement`)) 2.0) 1.0)) 1))
            (bind _output_get (set `self.CurrentAngle` (`KismetMathLibrary.MakeRotator` 0.0 0.0 (`self.CurrentYaw`))))
            (set `self.CurrentYaw` (- (`self.CurrentYaw`) (`self.SpreadIncrement`)))
            (`|SpawnActorFromClass` "/Game/Weapons/ShotgunWeapon/ShowgunShell.ShowgunShell_C" (`KismetMathLibrary.MakeTransform` (`SceneComponent.K2_GetComponentLocation` _arrow) (`KismetMathLibrary.ComposeRotators` _output_get (`self.GetSprayAngle` (`SceneComponent.GetForwardVector` _arrow)))) "Undefined" "MultiplyWithRoot" null (`self.ShellDamage`) (`self.Range`) null)))))))

(event `self.ReceiveBeginPlay`
  (`self.K2_AttachToActor` (`GameplayStatics.GetPlayerCharacter` 0) "None" "SnapToTarget" "KeepRelative" "KeepRelative")
  (set `self.Ammo` (`self.MagSize`))
  (`SphereComponent.SetSphereRadius` (`self.Sphere`) (`self.Range`) true))

(event `self.ReceiveTick`
  (params (DeltaSeconds :type "Float (single-precision)"))
  (`|ExecutionSequence`
    (:`then_0`
      (`self.GetClostestEnemy` (`PrimitiveComponent.GetOverlappingActors` (`self.Sphere`) "/Script/Engine.Character")))
    (:`then_1`
      (`self.CheckAmmo`))))

(event `CheckAmmo`
  (if (> (`self.Ammo`) 0.0)
    (`self.FireWeapon`)
    (else
      (set `self.Reloading` true)
      (bind _asbp_third_person_character (cast `/Game/ThirdPerson/Blueprints/BP_ThirdPersonCharacter` (`GameplayStatics.GetPlayerCharacter` 0)))
      (`KismetSystemLibrary.Delay` (* (- 1.0 (* (`BlueprintMapLibrary.Map_Find` (`/Game/ThirdPerson/Blueprints/BP_ThirdPersonCharacter.TempPlayerStats` _asbp_third_person_character) "ReloadSpeed") 0.01)) (`self.ReloadTime`)))
      (set `self.Ammo` (`self.MagSize`))
      (set `self.Reloading` false))))

(fn `GetClostestEnemy`
  (params (OverlappingActors :type "Array of Actor Object Reference"))
  (for _array_element OverlappingActors
    (if (`KismetSystemLibrary.DoesImplementInterface` _array_element "/Game/Interfaces/EnemyDetection.EnemyDetection_C")
      (`/Engine/EditorBlueprintResources/StandardMacros.IsValid` (`self.ClosestEnemy`)
        (:`Is Valid`
          (if (> (`KismetMathLibrary.VSize` (- (`self.K2_GetActorLocation` (`GameplayStatics.GetPlayerCharacter` 0)) (`self.K2_GetActorLocation` (`self.ClosestEnemy`)))) (`KismetMathLibrary.VSize` (- (`self.K2_GetActorLocation` (`GameplayStatics.GetPlayerCharacter` 0)) (`self.K2_GetActorLocation` _array_element))))
            (set `self.ClosestEnemy` _array_element)))
        (:`Is Not Valid`
          (set `self.ClosestEnemy` _array_element))))))

(fn `GetSprayAngle`
  (params (MuzzleDirection :type "Vector Structure"))
  (returns (ShotRotation :type "Rotator Structure"))
  (return (`KismetMathLibrary.MakeRotFromX` (`KismetMathLibrary.RandomUnitVectorInConeInDegrees` MuzzleDirection (`self.MaxRandomAngle`)))))

(fn `GetWeaponInfo`
  (returns (Image :type "Texture Object Reference") (Ammo :type "Float (double-precision)") (MagSize :type "Float (double-precision)") (Reloading :type Boolean))
  (return null (`self.Ammo`) (`self.MagSize`) (`self.Reloading`)))

(fn `UserConstructionScript`)