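; BP_Grenade is a grenade actor that explodes half a second after its sphere registers a hit.
; The explosion spawns an emitter scaled to the damage radius, applies full radial damage without falloff while ignoring the player, then destroys the actor.
; Damage gains a percentage bonus from the "Damage" entry in the player character's TempPlayerStats, so a failed character cast skips both damage and destruction.
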(event `self.Sphere.OnComponentHit`
  (params (HitComponent :type "PrimitiveComponent Object Reference") (OtherActor :type "Actor Object Reference") (OtherComp :type "PrimitiveComponent Object Reference") (NormalImpulse :type "Vector Structure") (Hit :type "HitResult Structure (by ref)"))
  (`KismetSystemLibrary.Delay` 0.5)
  (`GameplayStatics.SpawnEmitterAtLocation` "/Game/StarterContent/Particles/P_Explosion.P_Explosion" (`self.K2_GetActorLocation`) (struct) (`KismetMathLibrary.Conv_DoubleToVector` (/ (`self.DamageRadius`) 70.0)))
  (bind _asbp_third_person_character (cast `/Game/ThirdPerson/Blueprints/BP_ThirdPersonCharacter` (`GameplayStatics.GetPlayerCharacter` 0)))
  (`GameplayStatics.ApplyRadialDamage` (* (`self.Damage`) (+ (* (`BlueprintMapLibrary.Map_Find` (`/Game/ThirdPerson/Blueprints/BP_ThirdPersonCharacter.TempPlayerStats` _asbp_third_person_character) "Damage") 0.01) 1.0)) (`self.K2_GetActorLocation`) (`self.DamageRadius`) null (`|MakeArray` (`GameplayStatics.GetPlayerCharacter` 0) :!type "Actor Object Reference") null null true)
  (`self.K2_DestroyActor`))

(fn `UserConstructionScript`)