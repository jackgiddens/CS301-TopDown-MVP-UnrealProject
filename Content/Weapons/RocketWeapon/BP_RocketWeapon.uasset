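; Auto-firing rocket launcher attached to the player that targets the highest-health enemy within its range sphere.
; Enemy overlaps start and stop a looping fire timer, each shot launching a magazine-sized volley of homing rockets in a random upward cone.
; An empty magazine triggers a timeline reload, sped up by the player's ReloadSpeed stat.
; Damage comes from the weapons data table, and upgrades scale damage, fire rate or reload speed.
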(event `self.ReceiveBeginPlay`
  (bind _magsize (`self.MagSize`))
  (`self.K2_AttachToActor` (`GameplayStatics.GetPlayerCharacter` 0) "None" "SnapToTarget" "KeepRelative" "KeepRelative")
  (set `self.Ammo` _magsize)
  (set `self.RocketAmount` (`KismetMathLibrary.FTrunc` _magsize))
  (`SphereComponent.SetSphereRadius` (`self.Sphere`) (`self.Range`) true))

(event `StartFiring`
  (bind _returnvalue (`KismetSystemLibrary.K2_SetTimerDelegate` (delegate `CheckAmmo`) (`self.FireRate`) true))
  (set `self.FireWeaponTimer` _returnvalue))

(event `CheckAmmo`
  (if (`self.Reloading`)
    _
    (elif (> (`self.Ammo`) 0.0)
      (`self.FireWeapon`)
      (else
        (set `self.Reloading` true)
        (bind _asbp_third_person_character (cast `/Game/ThirdPerson/Blueprints/BP_ThirdPersonCharacter` (`GameplayStatics.GetPlayerCharacter` 0)))
        (`TimelineComponent.SetPlayRate` (`self.Reload`) (/ 1.0 (* (- 1.0 (* (`BlueprintMapLibrary.Map_Find` (`/Game/ThirdPerson/Blueprints/BP_ThirdPersonCharacter.TempPlayerStats` _asbp_third_person_character) "ReloadSpeed") 0.01)) (`self.ReloadSpeed`))))
        (bind (_direction _reload) (`Timeline|Reload` :!via `PlayFromStart`)
          (:`Update`
            (set `self.Ammo` (`KismetMathLibrary.Lerp` 0.0 (`self.MagSize`) _reload)))
          (:`Finished`
            (set `self.Reloading` false)))))))

(event `StopFiring`
  (set `self.IsFiring` false)
  (`KismetSystemLibrary.K2_ClearAndInvalidateTimerHandle` (`self.FireWeaponTimer`)))

(event `CheckOverlappingEnemies`
  (if (> (`KismetArrayLibrary.Array_Length` (`self.OverlappingEnemies`)) 0)
    (if (not (`self.IsFiring`))
      (set `self.IsFiring` true)
      (`self.StartFiring`))
    (else
      (`self.StopFiring`))))

(event `self.Sphere.OnComponentBeginOverlap`
  (params (OverlappedComponent :type "PrimitiveComponent Object Reference") (OtherActor :type "Actor Object Reference") (OtherComp :type "PrimitiveComponent Object Reference") (OtherBodyIndex :type Integer) (bFromSweep :type Boolean) (SweepResult :type "HitResult Structure (by ref)"))
  (if (`KismetSystemLibrary.DoesImplementInterface` OtherActor "/Game/Interfaces/EnemyDetection.EnemyDetection_C")
    (`KismetArrayLibrary.Array_Add` (`self.OverlappingEnemies`) OtherActor)
    (`self.CheckOverlappingEnemies`)))

(event `self.Sphere.OnComponentEndOverlap`
  (params (OverlappedComponent :type "PrimitiveComponent Object Reference") (OtherActor :type "Actor Object Reference") (OtherComp :type "PrimitiveComponent Object Reference") (OtherBodyIndex :type Integer))
  (if (`KismetSystemLibrary.DoesImplementInterface` OtherActor "/Game/Interfaces/EnemyDetection.EnemyDetection_C")
    (`KismetArrayLibrary.Array_RemoveItem` (`self.OverlappingEnemies`) OtherActor)
    (`self.CheckOverlappingEnemies`)))

(fn `FireWeapon`
  (bind _strongestenemy (`self.StrongestEnemy`))
  (bind _arrow (`self.Arrow`))
  (bind (_returnvalue_roll _returnvalue_pitch _returnvalue_yaw) (`KismetMathLibrary.BreakRotator` (`KismetMathLibrary.FindLookAtRotation` (`self.K2_GetActorLocation`) (`self.K2_GetActorLocation` (`self.StrongestEnemy`)))))
  (`self.GetStrongestEnemy` (`self.OverlappingEnemies`))
  (`/Engine/EditorBlueprintResources/StandardMacros.IsValid` (`self.StrongestEnemy`)
    (:`Is Valid`
      (if (< (`KismetMathLibrary.VSize` (- (`self.K2_GetActorLocation` (`GameplayStatics.GetPlayerCharacter` 0)) (`self.K2_GetActorLocation` (`self.StrongestEnemy`)))) (`self.Range`))
        (`SceneComponent.K2_SetWorldRotation` (`self.Arrow`) (`KismetMathLibrary.MakeRotator` _returnvalue_roll (+ _returnvalue_pitch 75.0) _returnvalue_yaw) false false)
        (for _ (range (`self.RocketAmount`))
          (bind _returnvalue (`|SpawnActorFromClass` "/Game/Weapons/RocketWeapon/BP_Rocket.BP_Rocket_C" (`KismetMathLibrary.MakeTransform` (`SceneComponent.K2_GetComponentLocation` _arrow) (`self.GetRocketAngle` (`SceneComponent.GetForwardVector` _arrow) (`self.MaxAngle`))) "Undefined" "MultiplyWithRoot" null (`self.RocketDamage`) (`self.StrongestEnemy`) null))
          (set `self.Ammo` (- (`self.Ammo`) 1.0))
          (`/Engine/EditorBlueprintResources/StandardMacros.IsValid` _strongestenemy
            (:`Is Valid`
              (set `ProjectileMovementComponent.HomingTargetComponent` (`Actor.RootComponent` _strongestenemy) (`/Game/Weapons/RocketWeapon/BP_Rocket.ProjectileMovement` _returnvalue)))
            (:`Is Not Valid`
              (`self.K2_DestroyActor` _returnvalue))))))))

(fn `GetRocketAngle`
  (params (Direction :type "Vector Structure") (MaxAngle :type "Float (double-precision)"))
  (returns (Rotation :type "Rotator Structure"))
  (return (`KismetMathLibrary.MakeRotFromX` (`KismetMathLibrary.RandomUnitVectorInConeInDegrees` Direction MaxAngle))))

(fn `GetStrongestEnemy`
  (params (OverlappingActors :type "Array of Actor Object Reference"))
  (for _array_element OverlappingActors
    (`/Engine/EditorBlueprintResources/StandardMacros.IsValid` (`self.StrongestEnemy`)
      (:`Is Valid`
        (if (`PrimitiveComponent.IsOverlappingActor` (`self.Sphere`) (`self.StrongestEnemy`))
          (bind _maxhealth (message `/Game/Interfaces/GetEnemyHealth.GetHealth` (`self.StrongestEnemy`)))
          (bind _maxhealth_2 (message `/Game/Interfaces/GetEnemyHealth.GetHealth` _array_element))
          (if (> _maxhealth_2 _maxhealth)
            (set `self.StrongestEnemy` _array_element))
          (else
            (set `self.StrongestEnemy` _array_element))))
      (:`Is Not Valid`
        (set `self.StrongestEnemy` _array_element)))))

(fn `GetWeaponInfo`
  (returns (Image :type "Texture2D Object Reference") (Ammo :type "Float (double-precision)") (MagSize :type "Float (double-precision)") (Reloading :type Boolean))
  (return "/Game/Weapons/RocketWeapon/RocketLauncherIcon.RocketLauncherIcon" (`self.Ammo`) (`self.MagSize`) (`self.Reloading`)))

(fn `UpgradeWeaponStats`
  (params (StatType :type String) (StatValue :type "Float (double-precision)"))
  (returns (bSuccess :type Boolean))
  (locals (StatValuePercent :type "Float (double-precision)"))
  (set `local.StatValuePercent` (* StatValue 0.01))
  (if (== StatType "WDamage")
    (set `self.RocketDamage` (* (+ (`local.StatValuePercent`) 1.0) (`self.RocketDamage`)))
    (elif (== StatType "WFireRate")
      (set `self.FireRate` (* (+ (`local.StatValuePercent`) 1.0) (`self.FireRate`)))
      (elif (== StatType "WReloadSpeed")
        (set `self.ReloadSpeed` (* (- 1.0 (`local.StatValuePercent`)) (`self.ReloadSpeed`)))
        (else
          (return false)))))
  (return true))

(fn `UserConstructionScript`
  (bind _returnvalue (`|GetDataTableRow` "/Game/Data/DataTables/WeaponsDataTable.WeaponsDataTable" "RocketWeapon")
    (:`then`
      (set `self.RocketDamage` (`.Damage_14_9E6566314152B3B1A7B2BAB456027CBA` (break `/Game/Data/Sturctures/Weapons` _returnvalue))))))