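; BP_Rocket is a rocket projectile that damages its Enemy actor on contact.
; When its capsule begins overlapping that actor, it spawns a half-scale explosion there, applies fire damage and destroys itself.
; Damage scales RocketDamage by the player character's TempPlayerStats Damage percentage, with a CritChance roll adding the CritDamage multiplier.
; Other overlaps are ignored, and no movement or targeting logic appears in its graphs.
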(event `self.Capsule.OnComponentBeginOverlap`
  (params (OverlappedComponent :type "PrimitiveComponent Object Reference") (OtherActor :type "Actor Object Reference") (OtherComp :type "PrimitiveComponent Object Reference") (OtherBodyIndex :type Integer) (bFromSweep :type Boolean) (SweepResult :type "HitResult Structure (by ref)"))
  ;[1 1 1] If rocket hits enemy deal damage
  (if (== OtherActor (`self.Enemy`))
    (`GameplayStatics.SpawnEmitterAtLocation` "/Game/StarterContent/Particles/P_Explosion.P_Explosion" (`self.K2_GetActorLocation` OtherActor) (struct) (0.5 0.5 0.5))
    (bind _asbp_third_person_character (cast `/Game/ThirdPerson/Blueprints/BP_ThirdPersonCharacter` (`GameplayStatics.GetPlayerCharacter` 0)))
    (bind _tempplayerstats (`/Game/ThirdPerson/Blueprints/BP_ThirdPersonCharacter.TempPlayerStats` _asbp_third_person_character))
    (bind _returnvalue (* (+ (* (`BlueprintMapLibrary.Map_Find` _tempplayerstats "Damage") 0.01) 1.0) (`self.RocketDamage`)))
    (`GameplayStatics.ApplyDamage` OtherActor (`KismetMathLibrary.SelectFloat` (* _returnvalue (+ (* (`BlueprintMapLibrary.Map_Find` _tempplayerstats "CritDamage") 0.01) 1.0)) _returnvalue (<= (`KismetMathLibrary.RandomFloatInRange` 0.0 1.0) (* (`BlueprintMapLibrary.Map_Find` _tempplayerstats "CritChance") 0.01))) null null "/Game/DamageTypes/DamageType_Fire.DamageType_Fire_C")
    (`self.K2_DestroyActor`)))

(fn `UserConstructionScript`)