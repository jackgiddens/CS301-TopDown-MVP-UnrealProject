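; Auto-firing flamethrower weapon that attaches to the player and burns enemies implementing EnemyDetection.
; A range sphere tracks enemies and, on overlap changes, schedules a next-tick turn of the Arrow toward the closest, stopping fire if none is in range.
; Enemies entering the box start a looping timer that spends ammo, applies fire damage scaled by player damage and crit stats, and reloads when empty.
; It also exposes weapon info and stat upgrades.
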(event `self.ReceiveBeginPlay`
  (bind _box (`self.Box`))
  (bind _range (`self.Range`))
  (bind _returnvalue (/ _range 2.0))
  (`self.K2_AttachToActor` (`GameplayStatics.GetPlayerCharacter` 0) "None" "SnapToTarget" "KeepRelative" "KeepRelative")
  (`SphereComponent.SetSphereRadius` (`self.Sphere`) _range true)
  (`SceneComponent.K2_SetRelativeLocation` _box (`KismetMathLibrary.MakeVector` _returnvalue) false false)
  (`BoxComponent.SetBoxExtent` _box (`KismetMathLibrary.MakeVector` _returnvalue 40.0 40.0) true)
  (set `self.Ammo` (`self.MagSize`)))

(event `StartDOT`
  (bind _returnvalue (`KismetSystemLibrary.K2_SetTimerDelegate` (delegate `DOT`) (`self.DamageTickRate`) true))
  (set `self.DOTTimer` _returnvalue))

(event `DOT`
  (bind _flamethrower (`self.FlameThrower`))
  (set `self.IsFiring` true)
  (if (> (`self.Ammo`) 0.0)
    (`ActorComponent.Activate` _flamethrower false)
    (set `self.Ammo` (- (`self.Ammo`) 1.0))
    (for _array_element (`PrimitiveComponent.GetOverlappingActors` (`self.Box`) "/Script/Engine.Character")
      (if (`KismetSystemLibrary.DoesImplementInterface` _array_element "/Game/Interfaces/EnemyDetection.EnemyDetection_C")
        (bind _asbp_third_person_character (cast `/Game/ThirdPerson/Blueprints/BP_ThirdPersonCharacter` (`GameplayStatics.GetPlayerCharacter` 0)))
        (bind _tempplayerstats (`/Game/ThirdPerson/Blueprints/BP_ThirdPersonCharacter.TempPlayerStats` _asbp_third_person_character))
        (bind _returnvalue (* (+ (* (`BlueprintMapLibrary.Map_Find` _tempplayerstats "Damage") 0.01) 1.0) (`self.FireDamage`)))
        (`GameplayStatics.ApplyDamage` _array_element (`KismetMathLibrary.SelectFloat` (* _returnvalue (+ (* (`BlueprintMapLibrary.Map_Find` _tempplayerstats "CritDamage") 0.01) 1.0)) _returnvalue (<= (`KismetMathLibrary.RandomFloatInRange` 0.0 1.0) (* (`BlueprintMapLibrary.Map_Find` _tempplayerstats "CritChance") 0.01))) null null "/Game/DamageTypes/DamageType_Fire.DamageType_Fire_C")))
    (else
      (`ActorComponent.Deactivate` _flamethrower)
      (`self.ReloadWeapon`))))

(event `EndDOT`
  (set `self.IsFiring` false)
  (`KismetSystemLibrary.K2_ClearAndInvalidateTimerHandle` (`self.DOTTimer`))
  (`ActorComponent.Deactivate` (`self.FlameThrower`)))

(event `CheckOverlappingEnemies`
  (if (> (`KismetArrayLibrary.Array_Length` (`self.OverlappingEnemies`)) 0)
    (bind _returnvalue (`KismetSystemLibrary.K2_SetTimerForNextTickDelegate` (delegate `SetWeaponRotation`)))
    (set `self.RotateTimer` _returnvalue)
    (else
      (`KismetSystemLibrary.K2_ClearAndInvalidateTimerHandle` (`self.RotateTimer`)))))

(event `SetWeaponRotation`
  (`self.GetClosestEnemy` (`self.OverlappingEnemies`))
  (`/Engine/EditorBlueprintResources/StandardMacros.IsValid` (`self.ClosestEnemy`)
    (:`Is Valid`
      (if (< (`KismetMathLibrary.VSize` (- (`self.K2_GetActorLocation` (`GameplayStatics.GetPlayerCharacter` 0)) (`self.K2_GetActorLocation` (`self.ClosestEnemy`)))) (`self.Range`))
        (`SceneComponent.K2_SetWorldRotation` (`self.Arrow`) (`KismetMathLibrary.FindLookAtRotation` (`self.K2_GetActorLocation`) (`self.K2_GetActorLocation` (`self.ClosestEnemy`))) false false)
        (else
          (`self.EndDOT`))))
    (:`Is Not Valid`
      (`self.EndDOT`))))

(event `ReloadWeapon`
  (set `self.Reloading` true)
  (bind _asbp_third_person_character (cast `/Game/ThirdPerson/Blueprints/BP_ThirdPersonCharacter` (`GameplayStatics.GetPlayerCharacter` 0)))
  (`ActorComponent.Deactivate` (`self.FlameThrower`))
  (`KismetSystemLibrary.Delay` (* (- 1.0 (* (`BlueprintMapLibrary.Map_Find` (`/Game/ThirdPerson/Blueprints/BP_ThirdPersonCharacter.TempPlayerStats` _asbp_third_person_character) "ReloadSpeed") 0.01)) (`self.ReloadSpeed`)))
  (set `self.Ammo` (`self.MagSize`))
  (set `self.Reloading` false))

(event `self.Box.OnComponentBeginOverlap`
  (params (OverlappedComponent :type "PrimitiveComponent Object Reference") (OtherActor :type "Actor Object Reference") (OtherComp :type "PrimitiveComponent Object Reference") (OtherBodyIndex :type Integer) (bFromSweep :type Boolean) (SweepResult :type "HitResult Structure (by ref)"))
  (if (`KismetSystemLibrary.DoesImplementInterface` OtherActor "/Game/Interfaces/EnemyDetection.EnemyDetection_C")
    (if (not (`self.IsFiring`))
      (`self.DOT`)
      (`self.StartDOT`))))

(event `self.Sphere.OnComponentBeginOverlap`
  (params (OverlappedComponent :type "PrimitiveComponent Object Reference") (OtherActor :type "Actor Object Reference") (OtherComp :type "PrimitiveComponent Object Reference") (OtherBodyIndex :type Integer) (bFromSweep :type Boolean) (SweepResult :type "HitResult Structure (by ref)"))
  (if (`KismetSystemLibrary.DoesImplementInterface` OtherActor "/Game/Interfaces/EnemyDetection.EnemyDetection_C")
    (`KismetArrayLibrary.Array_Add` (`self.OverlappingEnemies`) OtherActor)
    (`self.CheckOverlappingEnemies`)))

(event `self.Sphere.OnComponentEndOverlap`
  (params (OverlappedComponent :type "PrimitiveComponent Object Reference") (OtherActor :type "Actor Object Reference") (OtherComp :type "PrimitiveComponent Object Reference") (OtherBodyIndex :type Integer))
  (if (`KismetSystemLibrary.DoesImplementInterface` OtherActor "/Game/Interfaces/EnemyDetection.EnemyDetection_C")
    (`KismetArrayLibrary.Array_RemoveItem` (`self.OverlappingEnemies`) OtherActor)
    (`self.CheckOverlappingEnemies`)))

(fn `GetClosestEnemy`
  (params (OverlappingActors :type "Array of Actor Object Reference"))
  (for _array_element OverlappingActors
    (`/Engine/EditorBlueprintResources/StandardMacros.IsValid` (`self.ClosestEnemy`)
      (:`Is Valid`
        (if (> (`KismetMathLibrary.VSize` (- (`self.K2_GetActorLocation` (`GameplayStatics.GetPlayerCharacter` 0)) (`self.K2_GetActorLocation` (`self.ClosestEnemy`)))) (`KismetMathLibrary.VSize` (- (`self.K2_GetActorLocation` (`GameplayStatics.GetPlayerCharacter` 0)) (`self.K2_GetActorLocation` _array_element))))
          (set `self.ClosestEnemy` _array_element)))
      (:`Is Not Valid`
        (set `self.ClosestEnemy` _array_element)))))

(fn `GetWeaponInfo`
  (returns (Image :type "Texture2D Object Reference") (Ammo :type "Float (double-precision)") (MagSize :type "Float (double-precision)") (Reloading :type Boolean))
  (return "/Game/Weapons/FlamethrowerWeapon/FlamethrowerIcon.FlamethrowerIcon" (`self.Ammo`) (`self.MagSize`) (`self.Reloading`)))

(fn `UpgradeWeaponStats`
  (params (StatType :type String) (StatValue :type "Float (double-precision)"))
  (returns (bSuccess :type Boolean))
  (locals (StatValuePercent :type "Float (double-precision)"))
  (set `local.StatValuePercent` (* StatValue 0.01))
  (if (== StatType "WDamage")
    (set `self.FireDamage` (* (+ (`local.StatValuePercent`) 1.0) (`self.FireDamage`)))
    (elif (== StatType "WFireRate")
      (set `self.DamageTickRate` (* (+ (`local.StatValuePercent`) 1.0) (`self.DamageTickRate`)))
      (elif (== StatType "WReloadSpeed")
        (set `self.ReloadSpeed` (* (- (`local.StatValuePercent`) 1.0) (`self.ReloadSpeed`)))
        (else
          (return false)))))
  (return true))

(fn `UserConstructionScript`)