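; Auto-firing gun attached to the player character that shoots the nearest enemy in range and reports to the game HUD.
; Stats load from a data table row, with Range sizing the detection sphere that tracks EnemyDetection actors.
; A looping timer spawns bullets when a visibility trace is clear.
; A timeline refills ammo, scaled by the player's reload-speed stat, and upgrades adjust damage, fire rate and reload speed by percentage.
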(event `self.ReceiveBeginPlay`
  ;[1 1 1] Attach weapon to Character, get refernce to game hud and update weapon UI
  (`self.K2_AttachToActor` (`GameplayStatics.GetPlayerCharacter` 0) "None" "SnapToTarget" "KeepRelative" "KeepRelative")
  (`self.SetStats`)
  (`KismetSystemLibrary.Delay` 0.2)
  (bind _asbp_game_hud (cast `/Game/ThirdPerson/Blueprints/BP_GameHUD` (`PlayerController.GetHUD` (`GameplayStatics.GetPlayerController` 0))))
  (bind _output_get (set `self.Game HUD` (`/Game/ThirdPerson/Blueprints/BP_GameHUD.GameHUD` _asbp_game_hud)))
  (message `/Game/Interfaces/UpdateHUD.UpdateWeapons` _output_get self)
  (message `/Game/Interfaces/UpdateHUD.UpdateWeaponSlots` _output_get))

(event `CheckOverlappingEnemies`
  ;[1 1 1] Check overlapping enemies array if lenght > 0 and gun is not firing start firing weapon
  (if (> (`KismetArrayLibrary.Array_Length` (`self.OverlappingEnemies`)) 0)
    (if (not (`self.IsFiring`))
      (set `self.IsFiring` true)
      (`self.CheckAmmo`)
      (`self.StartFiring`))
    (else
      (`self.StopFiring`))))

(event `StartFiring`
  ;[1 1 1] Firing Timer
  (bind _returnvalue (`KismetSystemLibrary.K2_SetTimerDelegate` (delegate `CheckAmmo`) (`self.FireRate`) true))
  (set `self.FireWeaponTimer` _returnvalue))

(event `CheckAmmo`
  ;[1 1 1] Firing Timer
  (if (`self.Reloading`)
    _
    (elif (> (`self.Ammo`) 0.0)
      (`self.FireWeapon`)
      (message `/Game/Interfaces/UpdateHUD.UpdateWeaponSlots` (`self.Game HUD`))
      (else
        (`self.ReloadWeapon`)))))

(event `ReloadWeapon`
  ;[1 1 1] Reload Weapon
  (set `self.Reloading` true)
  (bind _asbp_third_person_character (cast `/Game/ThirdPerson/Blueprints/CharacterClasses/BP_BaseCharacter` (`GameplayStatics.GetPlayerCharacter` 0)))
  (`TimelineComponent.SetPlayRate` (`self.Reload`) (/ 1.0 (* (- 1.0 (* (`BlueprintMapLibrary.Map_Find` (`/Game/ThirdPerson/Blueprints/CharacterClasses/BP_BaseCharacter.TempPlayerStats` _asbp_third_person_character) "ReloadSpeed") 0.01)) (`self.ReloadSpeed`))))
  (bind (_direction _reload) (`Timeline|Reload` :!via `PlayFromStart`)
    (:`Update`
      (set `self.Ammo` (`KismetMathLibrary.Lerp` 0.0 (`self.MagSize`) _reload))
      (`KismetSystemLibrary.Delay` 0.2)
      (message `/Game/Interfaces/UpdateHUD.UpdateWeaponSlots` (`self.Game HUD`)))
    (:`Finished`
      (set `self.Reloading` false))))

(event `StopFiring`
  ;[1 1 1] Stop firing timer
  (set `self.IsFiring` false)
  (`KismetSystemLibrary.K2_ClearAndInvalidateTimerHandle` (`self.FireWeaponTimer`)))

(event `self.Sphere.OnComponentBeginOverlap`
  (params (OverlappedComponent :type "PrimitiveComponent Object Reference") (OtherActor :type "Actor Object Reference") (OtherComp :type "PrimitiveComponent Object Reference") (OtherBodyIndex :type Integer) (bFromSweep :type Boolean) (SweepResult :type "HitResult Structure (by ref)"))
  ;[1 1 1] Added enemies within range to overlapping enemies array
  (if (`KismetSystemLibrary.DoesImplementInterface` OtherActor "/Game/Interfaces/EnemyDetection.EnemyDetection_C")
    (`KismetArrayLibrary.Array_Add` (`self.OverlappingEnemies`) OtherActor)
    (`self.CheckOverlappingEnemies`)))

(event `self.Sphere.OnComponentEndOverlap`
  (params (OverlappedComponent :type "PrimitiveComponent Object Reference") (OtherActor :type "Actor Object Reference") (OtherComp :type "PrimitiveComponent Object Reference") (OtherBodyIndex :type Integer))
  ;[1 1 1] Removes enemies that leave range from overlapping enemies
  (if (`KismetSystemLibrary.DoesImplementInterface` OtherActor "/Game/Interfaces/EnemyDetection.EnemyDetection_C")
    (`KismetArrayLibrary.Array_RemoveItem` (`self.OverlappingEnemies`) OtherActor)
    (`KismetSystemLibrary.Delay` (`KismetSystemLibrary.K2_GetTimerRemainingTimeHandle` (`self.FireWeaponTimer`)))
    (`self.CheckOverlappingEnemies`)))

(fn `FireWeapon`
  ;[1 1 1] Fires weapon at closest enemy
  (`self.GetClosestEnemy` (`self.OverlappingEnemies`))
  (`/Engine/EditorBlueprintResources/StandardMacros.IsValid` (`self.ClosestEnemy`)
    (:`Is Valid`
      (bind (_outhit _returnvalue) (`KismetSystemLibrary.LineTraceSingle` (`self.K2_GetActorLocation` (`GameplayStatics.GetPlayerCharacter` 0)) (`self.K2_GetActorLocation` (`self.ClosestEnemy`)) "TraceTypeQuery1"))
      (if _returnvalue
        _
        (elif (< (`KismetMathLibrary.VSize` (- (`self.K2_GetActorLocation` (`GameplayStatics.GetPlayerCharacter` 0)) (`self.K2_GetActorLocation` (`self.ClosestEnemy`)))) (`self.Range`))
          (`SceneComponent.K2_SetWorldRotation` (`self.Arrow`) (`KismetMathLibrary.FindLookAtRotation` (`self.K2_GetActorLocation`) (`self.K2_GetActorLocation` (`self.ClosestEnemy`))) false false)
          (`|SpawnActorFromClass` "/Game/NewWeapons/New_Weapons/AssaultWeapon/BP_MachineGunBullet.BP_MachineGunBullet_C" (`SceneComponent.K2_GetComponentToWorld` (`self.Arrow`)) "Undefined" "MultiplyWithRoot" null (`self.BulletDamage`) null)
          (bind _output_get (set `self.Ammo` (- (`self.Ammo`) 1.0)))
          (if (== _output_get 0.0)
            (`self.ReloadWeapon`)))))))

(fn `GetClosestEnemy`
  (params (OverlappingActors :type "Array of Actor Object Reference"))
  ;[1 1 1] Get closest enemy to player
  (for _array_element OverlappingActors
    (`/Engine/EditorBlueprintResources/StandardMacros.IsValid` (`self.ClosestEnemy`)
      (:`Is Valid`
        (if (> (`KismetMathLibrary.VSize` (- (`self.K2_GetActorLocation` (`GameplayStatics.GetPlayerCharacter` 0)) (`self.K2_GetActorLocation` (`self.ClosestEnemy`)))) (`KismetMathLibrary.VSize` (- (`self.K2_GetActorLocation` (`GameplayStatics.GetPlayerCharacter` 0)) (`self.K2_GetActorLocation` _array_element))))
          (set `self.ClosestEnemy` _array_element)))
      (:`Is Not Valid`
        (set `self.ClosestEnemy` _array_element)))))

(fn `GetWeaponInfo`
  (returns (Image :type "Texture2D Object Reference") (Ammo :type "Float (double-precision)") (MagSize :type "Float (double-precision)") (Reloading :type Boolean))
  ;[1 1 1] Get Weapon Info
  (return "/Game/NewWeapons/New_Weapons/AssaultWeapon/MachineGunIcon.MachineGunIcon" (`self.Ammo`) (`self.MagSize`) (`self.Reloading`)))

(fn `SetStats`
  ;[1 1 1] Sets weapon stats from datatable
  (bind _returnvalue (`|GetDataTableRow` "/Game/Data/DataTables/WeaponsDataTable.WeaponsDataTable" "SimpleGunWeapon")
    (:`then`
      (bind (_weaponname _damage _reloadspeed _firerate _magsize _range) (break `/Game/Data/Sturctures/Weapons` _returnvalue))
      (set `self.BulletDamage` _damage)
      (set `self.ReloadSpeed` _reloadspeed)
      (set `self.FireRate` _firerate)
      (bind _output_get (set `self.MagSize` _magsize))
      (bind _output_get_2 (set `self.Range` _range))
      (`SphereComponent.SetSphereRadius` (`self.Sphere`) _output_get_2 true)
      (set `self.Ammo` _output_get))))

(fn `UpgradeWeaponStats`
  (params (StatType :type String) (StatValue :type "Float (double-precision)"))
  (returns (bSuccess :type Boolean))
  (locals (StatValuePercent :type "Float (double-precision)"))
  ;[1 1 1] Upgrades weapons stats
  (set `local.StatValuePercent` (* StatValue 0.01))
  (if (== StatType "WDamage")
    (set `self.BulletDamage` (* (+ (`local.StatValuePercent`) 1.0) (`self.BulletDamage`)))
    (elif (== StatType "WFireRate")
      (set `self.FireRate` (* (+ (`local.StatValuePercent`) 1.0) (`self.FireRate`)))
      (elif (== StatType "WReloadSpeed")
        (set `self.ReloadSpeed` (* (- 1.0 (`local.StatValuePercent`)) (`self.ReloadSpeed`)))
        (else
          (return false)))))
  (return true))

(fn `UserConstructionScript`)