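; Auto-aiming flamethrower weapon that attaches to the player and burns overlapping enemies.
; Construction loads data table stats, sizes the range sphere and flame box, and scales damage and reload time by player level.
; Sphere overlaps drive a timer that turns the arrow toward the closest enemy, while box overlaps start looping fire damage using player crit stats.
; Ammo refills through a reload timeline, the HUD shows weapon state, and upgrades modify stats.
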(event `self.ReceiveBeginPlay`
  ;[1 1 1] Attach weapon to Character, get refernce to game hud and update weapon UI
  (`self.K2_AttachToActor` (`GameplayStatics.GetPlayerCharacter` 0) "None" "SnapToTarget" "KeepRelative" "KeepRelative")
  (`KismetSystemLibrary.Delay` 0.2)
  (bind _asbp_game_hud (cast `/Game/ThirdPerson/Blueprints/BP_GameHUD` (`PlayerController.GetHUD` (`GameplayStatics.GetPlayerController` 0))))
  (bind _output_get (set `self.Game HUD` (`/Game/ThirdPerson/Blueprints/BP_GameHUD.GameHUD` _asbp_game_hud)))
  (message `/Game/Interfaces/UpdateHUD.UpdateWeapons` _output_get self)
  (message `/Game/Interfaces/UpdateHUD.UpdateWeaponSlots` _output_get))

(event `StartDOT`
  ;[1 1 1] Start damage over time timer and applies damage to overlapping actors with fire
  (bind _returnvalue (`KismetSystemLibrary.K2_SetTimerDelegate` (delegate `DOT`) (`self.DamageTickRate`) true))
  (set `self.DOTTimer` _returnvalue))

(event `DOT`
  (bind _flamethrower (`self.FlameThrower`))
  ;[1 1 1] Start damage over time timer and applies damage to overlapping actors with fire
  (set `self.IsFiring` true)
  (if (`self.Reloading`)
    _
    (elif (> (`self.Ammo`) 0.0)
      (`ActorComponent.Activate` _flamethrower false)
      (set `self.Ammo` (- (`self.Ammo`) 1.0))
      (for _array_element (`PrimitiveComponent.GetOverlappingActors` (`self.Box`) "/Script/Engine.Character")
        (if (`KismetSystemLibrary.DoesImplementInterface` _array_element "/Game/Interfaces/EnemyDetection.EnemyDetection_C")
          (bind _asbp_third_person_character (cast `/Game/ThirdPerson/Blueprints/BP_ThirdPersonCharacter` (`GameplayStatics.GetPlayerCharacter` 0)))
          (bind _tempplayerstats (`/Game/ThirdPerson/Blueprints/BP_ThirdPersonCharacter.TempPlayerStats` _asbp_third_person_character))
          (bind _returnvalue (* (+ (* (`BlueprintMapLibrary.Map_Find` _tempplayerstats "Damage") 0.01) 1.0) (`self.FireDamage`)))
          (`GameplayStatics.ApplyDamage` _array_element (`KismetMathLibrary.SelectFloat` (* _returnvalue (+ (* (`BlueprintMapLibrary.Map_Find` _tempplayerstats "CritDamage") 0.01) 1.0)) _returnvalue (<= (`KismetMathLibrary.RandomFloatInRange` 0.0 1.0) (* (`BlueprintMapLibrary.Map_Find` _tempplayerstats "CritChance") 0.01))) null null "/Game/DamageTypes/DamageType_Fire.DamageType_Fire_C")
          (message `/Game/Interfaces/UpdateHUD.UpdateWeaponSlots` (`self.Game HUD`))
          (if (== (`self.Ammo`) 0.0)
            (`self.ReloadWeapon`))))
      (else
        (`ActorComponent.Deactivate` _flamethrower)
        (`self.ReloadWeapon`)))))

(event `EndDOT`
  ;[1 1 1] Start damage over time timer and applies damage to overlapping actors with fire
  ;;[1 1 1] End damage over time timer
  (set `self.IsFiring` false)
  (`KismetSystemLibrary.K2_ClearAndInvalidateTimerHandle` (`self.DOTTimer`))
  (`ActorComponent.Deactivate` (`self.FlameThrower`)))

(event `CheckOverlappingEnemies`
  ;[1 1 1] Sets weapon rotation towards closest enemy
  (if (> (`KismetArrayLibrary.Array_Length` (`self.OverlappingEnemies`)) 0)
    (bind _returnvalue (`KismetSystemLibrary.K2_SetTimerDelegate` (delegate `SetWeaponRotation`) 0.2 true))
    (set `self.RotateTimer` _returnvalue)
    (else
      (`KismetSystemLibrary.K2_ClearAndInvalidateTimerHandle` (`self.RotateTimer`))
      (`self.EndDOT`))))

(event `SetWeaponRotation`
  ;[1 1 1] Sets weapon rotation towards closest enemy
  (`self.GetClosestEnemy` (`self.OverlappingEnemies`))
  (`/Engine/EditorBlueprintResources/StandardMacros.IsValid` (`self.ClosestEnemy`)
    (:`Is Valid`
      (if (< (`KismetMathLibrary.VSize` (- (`self.K2_GetActorLocation` (`GameplayStatics.GetPlayerCharacter` 0)) (`self.K2_GetActorLocation` (`self.ClosestEnemy`)))) (`self.Range`))
        (`SceneComponent.K2_SetWorldRotation` (`self.Arrow`) (`KismetMathLibrary.FindLookAtRotation` (`self.K2_GetActorLocation`) (`self.K2_GetActorLocation` (`self.ClosestEnemy`))) false false)
        (else
          (`self.EndDOT`))))
    (:`Is Not Valid`
      (`self.EndDOT`))))

(event `ReloadWeapon`
  ;[1 1 1] Reload Weapon
  (set `self.Reloading` true)
  (bind _asbp_third_person_character (cast `/Game/ThirdPerson/Blueprints/BP_ThirdPersonCharacter` (`GameplayStatics.GetPlayerCharacter` 0)))
  (`ActorComponent.Deactivate` (`self.FlameThrower`))
  (`TimelineComponent.SetPlayRate` (`self.Reload`) (/ 1.0 (* (- 1.0 (* (`BlueprintMapLibrary.Map_Find` (`/Game/ThirdPerson/Blueprints/BP_ThirdPersonCharacter.TempPlayerStats` _asbp_third_person_character) "ReloadSpeed") 0.01)) (`self.ReloadSpeed`))))
  (bind (_direction _reload) (`Timeline|Reload` :!via `PlayFromStart`)
    (:`Update`
      (set `self.Ammo` (`KismetMathLibrary.Lerp` 0.0 (`self.MagSize`) _reload))
      (`KismetSystemLibrary.Delay` 0.2)
      (message `/Game/Interfaces/UpdateHUD.UpdateWeaponSlots` (`self.Game HUD`)))
    (:`Finished`
      (set `self.Reloading` false))))

(event `self.Box.OnComponentBeginOverlap`
  (params (OverlappedComponent :type "PrimitiveComponent Object Reference") (OtherActor :type "Actor Object Reference") (OtherComp :type "PrimitiveComponent Object Reference") (OtherBodyIndex :type Integer) (bFromSweep :type Boolean) (SweepResult :type "HitResult Structure (by ref)"))
  ;[1 1 1] If enemies overlap fire deal damage over time
  (if (`KismetSystemLibrary.DoesImplementInterface` OtherActor "/Game/Interfaces/EnemyDetection.EnemyDetection_C")
    (if (not (`self.IsFiring`))
      (`self.DOT`)
      (`self.StartDOT`))))

(event `self.Sphere.OnComponentBeginOverlap`
  (params (OverlappedComponent :type "PrimitiveComponent Object Reference") (OtherActor :type "Actor Object Reference") (OtherComp :type "PrimitiveComponent Object Reference") (OtherBodyIndex :type Integer) (bFromSweep :type Boolean) (SweepResult :type "HitResult Structure (by ref)"))
  ;[1 1 1] Added enemies within range to overlapping enemies array
  (if (`KismetSystemLibrary.DoesImplementInterface` OtherActor "/Game/Interfaces/EnemyDetection.EnemyDetection_C")
    (`KismetArrayLibrary.Array_Add` (`self.OverlappingEnemies`) OtherActor)
    (`self.CheckOverlappingEnemies`)))

(event `self.Sphere.OnComponentEndOverlap`
  (params (OverlappedComponent :type "PrimitiveComponent Object Reference") (OtherActor :type "Actor Object Reference") (OtherComp :type "PrimitiveComponent Object Reference") (OtherBodyIndex :type Integer))
  ;[1 1 1] Removes enemies that leave range from overlapping enemies
  (if (`KismetSystemLibrary.DoesImplementInterface` OtherActor "/Game/Interfaces/EnemyDetection.EnemyDetection_C")
    (`KismetArrayLibrary.Array_RemoveItem` (`self.OverlappingEnemies`) OtherActor)
    (`self.CheckOverlappingEnemies`)))

(fn `GetClosestEnemy`
  (params (OverlappingActors :type "Array of Actor Object Reference"))
  ;[1 1 1] Gets closest enemy to player
  (for _array_element OverlappingActors
    (`/Engine/EditorBlueprintResources/StandardMacros.IsValid` (`self.ClosestEnemy`)
      (:`Is Valid`
        (if (> (`KismetMathLibrary.VSize` (- (`self.K2_GetActorLocation` (`GameplayStatics.GetPlayerCharacter` 0)) (`self.K2_GetActorLocation` (`self.ClosestEnemy`)))) (`KismetMathLibrary.VSize` (- (`self.K2_GetActorLocation` (`GameplayStatics.GetPlayerCharacter` 0)) (`self.K2_GetActorLocation` _array_element))))
          (set `self.ClosestEnemy` _array_element)))
      (:`Is Not Valid`
        (set `self.ClosestEnemy` _array_element)))))

(fn `GetWeaponInfo`
  (returns (Image :type "Texture2D Object Reference") (Ammo :type "Float (double-precision)") (MagSize :type "Float (double-precision)") (Reloading :type Boolean))
  ;[1 1 1] Get Weapon Info
  (return "/Game/NewWeapons/New_Weapons/FlameThrowerWeapon/FlamethrowerIcon.FlamethrowerIcon" (`self.Ammo`) (`self.MagSize`) (`self.Reloading`)))

(fn `ScaleStats`
  ;[1 1 1] When weapon spawns scale stats based on player level
  (bind _asbp_third_person_character (cast `/Game/ThirdPerson/Blueprints/BP_ThirdPersonCharacter` (`GameplayStatics.GetPlayerCharacter` 0)))
  (bind _returnvalue (+ (* (`KismetMathLibrary.Conv_IntToDouble` (`/Game/ThirdPerson/Blueprints/BP_ThirdPersonCharacter.Level` _asbp_third_person_character)) 0.05) 1.0))
  (set `self.FireDamage` (* _returnvalue (`self.FireDamage`)))
  (set `self.ReloadSpeed` (* _returnvalue (`self.ReloadSpeed`))))

(fn `UpgradeWeaponStats`
  (params (StatType :type String) (StatValue :type "Float (double-precision)"))
  (returns (bSuccess :type Boolean))
  (locals (StatValuePercent :type "Float (double-precision)"))
  ;[1 1 1] Upgrades weapons stats
  (set `local.StatValuePercent` (* StatValue 0.01))
  (if (== StatType "WDamage")
    (set `self.FireDamage` (* (+ (`local.StatValuePercent`) 1.0) (`self.FireDamage`)))
    (elif (== StatType "WFireRate")
      (set `self.DamageTickRate` (* (+ (`local.StatValuePercent`) 1.0) (`self.DamageTickRate`)))
      (elif (== StatType "WReloadSpeed")
        (set `self.ReloadSpeed` (* (- 1.0 (`local.StatValuePercent`)) (`self.ReloadSpeed`)))
        (else
          (return false)))))
  (return true))

(fn `UserConstructionScript`
  (bind _box (`self.Box`))
  ;[1 1 1] Sets weapon stats from datatable and set collision box location and extent
  (bind _returnvalue (`|GetDataTableRow` "/Game/Data/DataTables/WeaponsDataTable.WeaponsDataTable" "FlameThrower")
    (:`then`
      (bind (_weaponname _damage _reloadspeed _firerate _magsize _range) (break `/Game/Data/Sturctures/Weapons` _returnvalue))
      (set `self.FireDamage` _damage)
      (set `self.ReloadSpeed` _reloadspeed)
      (set `self.DamageTickRate` _firerate)
      (bind _output_get (set `self.MagSize` _magsize))
      (bind _output_get_2 (set `self.Range` _range))
      (`SphereComponent.SetSphereRadius` (`self.Sphere`) _output_get_2 true)
      (bind _returnvalue_2 (/ _output_get_2 2.0))
      (`SceneComponent.K2_SetRelativeLocation` _box (`KismetMathLibrary.MakeVector` _returnvalue_2) false false)
      (`BoxComponent.SetBoxExtent` _box (`KismetMathLibrary.MakeVector` _returnvalue_2 40.0 40.0) true)
      (set `self.Ammo` _output_get)
      (`self.ScaleStats`))))