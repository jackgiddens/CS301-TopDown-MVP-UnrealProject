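; Base auto-firing weapon actor that attaches to the player, with an empty FireWeapon for child weapons to override.
; Data table stats set damage, timings, magazine and range sphere radius, with functions for level scaling and upgrades.
; Enemies overlapping the sphere drive a looping fire timer; an empty magazine triggers a timeline reload, rate-adjusted by player stats, that refills ammo.
; Helpers provide closest or highest-health targeting and line-of-sight checks, while HUD messages update weapon slots.
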(event `IsOverlappingWhenSpawned`
  (bind _overlappingactors (`PrimitiveComponent.GetOverlappingActors` (`self.BP_Sphere`) "/Game/Enemies/BP_BaseEnemies.BP_BaseEnemies_C"))
  (`KismetSystemLibrary.Delay` 0.2)
  (if (`KismetArrayLibrary.Array_IsValidIndex` _overlappingactors)
    (`KismetArrayLibrary.Array_AddUnique` _overlappingactors)
    (`self.CheckOverlappingEnemies`)))

(event `self.ReceiveBeginPlay`
  (`self.K2_AttachToActor` (`GameplayStatics.GetPlayerCharacter` 0) "None" "SnapToTarget" "KeepRelative" "KeepRelative")
  (`self.SetStats` "Error")
  (set `self.IsFiring` false) ; So weapon doesnt try to fire before ammo is set
  (bind _asbp_base_character (cast `/Game/ThirdPerson/Blueprints/CharacterClasses/BP_BaseCharacter` (`GameplayStatics.GetPlayerCharacter` 0)))
  (set `self.CharREF` _asbp_base_character)
  (`KismetSystemLibrary.Delay` 0.2)
  (`self.IsOverlappingWhenSpawned`)
  (bind _asbp_game_hud (cast `/Game/ThirdPerson/Blueprints/BP_GameHUD` (`PlayerController.GetHUD` (`GameplayStatics.GetPlayerController` 0))))
  (bind _output_get (set `self.Game HUD` (`/Game/ThirdPerson/Blueprints/BP_GameHUD.GameHUD` _asbp_game_hud)))
  (message `/Game/Interfaces/UpdateHUD.UpdateWeapons` _output_get self)
  (message `/Game/Interfaces/UpdateHUD.UpdateWeaponSlots` _output_get)
  (set `self.Reloading` false))

(event `self.BP_Sphere.OnComponentBeginOverlap`
  (params (OverlappedComponent :type "PrimitiveComponent Object Reference") (OtherActor :type "Actor Object Reference") (OtherComp :type "PrimitiveComponent Object Reference") (OtherBodyIndex :type Integer) (bFromSweep :type Boolean) (SweepResult :type "HitResult Structure (by ref)"))
  (bind _asbp_base_enemies (cast `/Game/Enemies/BP_BaseEnemies` OtherActor))
  (`KismetArrayLibrary.Array_AddUnique` (`self.OverlappingEnemies`) _asbp_base_enemies)
  (`self.CheckOverlappingEnemies`))

(event `self.BP_Sphere.OnComponentEndOverlap`
  (params (OverlappedComponent :type "PrimitiveComponent Object Reference") (OtherActor :type "Actor Object Reference") (OtherComp :type "PrimitiveComponent Object Reference") (OtherBodyIndex :type Integer))
  (bind _asbp_base_enemies (cast `/Game/Enemies/BP_BaseEnemies` OtherActor))
  (`KismetArrayLibrary.Array_RemoveItem` (`self.OverlappingEnemies`) _asbp_base_enemies)
  (`KismetSystemLibrary.Delay` (`KismetSystemLibrary.K2_GetTimerRemainingTimeHandle` (`self.FireWeaponTimer`)))
  (`self.CheckOverlappingEnemies`))

(event `CheckOverlappingEnemies`
  (if (> (`KismetArrayLibrary.Array_Length` (`self.OverlappingEnemies`)) 0)
    (if (not (`self.IsFiring`))
      (set `self.IsFiring` true)
      (`self.CheckAmmo`)
      (`self.StartFireWeapon`))
    (else
      (`self.StopFiringWeapon`))))

(event `StartFireWeapon`
  (bind _returnvalue (`KismetSystemLibrary.K2_SetTimerDelegate` (delegate `CheckAmmo`) (`self.FireRate`) true))
  (set `self.FireWeaponTimer` _returnvalue))

(event `CheckAmmo`
  (if (`self.Reloading`)
    _
    (elif (> (`self.Ammo`) 0.0)
      (`self.FireWeapon`)
      (message `/Game/Interfaces/UpdateHUD.UpdateWeaponSlots` (`self.Game HUD`))
      (else
        (`self.ReloadWeapon`)))))

(event `StopFiringWeapon`
  (set `self.IsFiring` false)
  (`KismetSystemLibrary.K2_ClearAndInvalidateTimerHandle` (`self.FireWeaponTimer`)))

(event `ReloadWeapon`
  (set `self.Reloading` true)
  (bind _asbp_base_character (cast `/Game/ThirdPerson/Blueprints/CharacterClasses/BP_BaseCharacter` (`GameplayStatics.GetPlayerCharacter` 0)))
  (`TimelineComponent.SetPlayRate` (`self.ReloadTimeline`) (/ 1.0 (* (- 1.0 (* (`BlueprintMapLibrary.Map_Find` (`/Game/ThirdPerson/Blueprints/CharacterClasses/BP_BaseCharacter.TempPlayerStats` _asbp_base_character) "ReloadSpeed") 0.01)) (`self.ReloadSpeed`))))
  (bind (_direction _reload) (`Timeline|ReloadTimeline` :!via `PlayFromStart`)
    (:`Update`
      (set `self.Ammo` (`KismetMathLibrary.Lerp` 0.0 (`self.MagSize`) _reload))
      (`KismetSystemLibrary.Delay` 0.2)
      (message `/Game/Interfaces/UpdateHUD.UpdateWeaponSlots` (`self.Game HUD`)))
    (:`Finished`
      (set `self.Reloading` false))))

(fn `BP_GetClosestEnemy`
  (params (OverlappingActors :type "Array of Actor Object Reference"))
  (locals (ClosestEnemy :type "Actor Object Reference"))
  (bind _targetenemy (`self.TargetEnemy`))
  ;[1 1 1] Get closest enemy to player
  (for _array_element OverlappingActors
    (`/Engine/EditorBlueprintResources/StandardMacros.IsValid` _targetenemy
      (:`Is Valid`
        (if (> (`KismetMathLibrary.VSize` (- (`self.K2_GetActorLocation` (`GameplayStatics.GetPlayerCharacter` 0)) (`self.K2_GetActorLocation` _targetenemy))) (`KismetMathLibrary.VSize` (- (`self.K2_GetActorLocation` (`GameplayStatics.GetPlayerCharacter` 0)) (`self.K2_GetActorLocation` _array_element))))
          (set `self.TargetEnemy` _array_element)))
      (:`Is Not Valid`
        (set `self.TargetEnemy` _array_element)))))

(fn `BP_GetStrongestEnemy`
  (params (OverlappingActors :type "Array of Actor Object Reference"))
  ;[1 1 1] Gets enemy with most health
  (for _array_element OverlappingActors
    (`/Engine/EditorBlueprintResources/StandardMacros.IsValid` (`self.TargetEnemy`)
      (:`Is Valid`
        (if (`PrimitiveComponent.IsOverlappingActor` (`self.BP_Sphere`) (`self.TargetEnemy`))
          (bind _maxhealth (message `/Game/Interfaces/GetEnemyHealth.GetHealth` (`self.TargetEnemy`)))
          (bind _maxhealth_2 (message `/Game/Interfaces/GetEnemyHealth.GetHealth` _array_element))
          (if (> _maxhealth_2 _maxhealth)
            (set `self.TargetEnemy` _array_element))
          (else
            (set `self.TargetEnemy` _array_element))))
      (:`Is Not Valid`
        (set `self.TargetEnemy` _array_element)))))

(fn `FireWeapon`)

(fn `GetWeaponInfo`
  (returns (Image :type "Texture2D Object Reference") (Ammo :type "Float (double-precision)") (MagSize :type "Float (double-precision)") (Reloading :type Boolean))
  (return null 0.0 0.0 false))

(fn `IsInLineOfSight`
  (params (Enemy :type "Actor Object Reference") (Range :type "Float (double-precision)"))
  (returns (IsInRange :type Boolean))
  (bind (_outhit _returnvalue) (`KismetSystemLibrary.LineTraceSingle` (`self.K2_GetActorLocation` (`GameplayStatics.GetPlayerCharacter` 0)) (`self.K2_GetActorLocation` Enemy) "TraceTypeQuery1"))
  (if _returnvalue
    (return false)
    (else
      (return true))))

(fn `ScaleStats`
  (params (ScaleAmt :type "Float (double-precision)"))
  (bind _returnvalue (+ (* (`KismetMathLibrary.Conv_IntToDouble` (`/Game/ThirdPerson/Blueprints/CharacterClasses/BP_BaseCharacter.Level` (`self.CharREF`))) 0.05) 1.0))
  ;[1 1 1] When weapon spawns scale stats based on player level
  (set `self.Damage` (* _returnvalue (`self.Damage`)))
  (set `self.FireRate` (* _returnvalue (`self.FireRate`)))
  (set `self.ReloadSpeed` (* _returnvalue (`self.ReloadSpeed`))))

(fn `SetStats`
  (params (RowName :type Name))
  ;[1 1 1] Sets weapon stats from datatable
  (bind _returnvalue (`|GetDataTableRow` "/Game/Data/DataTables/WeaponsDataTable.WeaponsDataTable" RowName)
    (:`then`
      (bind (_weaponname _damage _reloadspeed _firerate _magsize _range) (break `/Game/Data/Sturctures/Weapons` _returnvalue))
      (set `self.Damage` _damage)
      (set `self.ReloadSpeed` _reloadspeed)
      (set `self.FireRate` _firerate)
      (bind _output_get (set `self.MagSize` _magsize))
      (bind _output_get_2 (set `self.Range` _range))
      (`SphereComponent.SetSphereRadius` (`self.BP_Sphere`) _output_get_2 true)
      (set `self.Ammo` _output_get))
    (:`RowNotFound`
      (`KismetSystemLibrary.PrintString` "Row Not Found!"))))

(fn `UpgradeWeaponStats`
  (params (StatType :type String) (StatValue :type "Float (double-precision)"))
  (returns (bSuccess :type Boolean))
  (locals (StatValuePercent :type "Float (double-precision)"))
  ;[1 1 1] Upgrades weapons stats
  (set `local.StatValuePercent` (* StatValue 0.01))
  (if (== StatType "WDamage")
    (set `self.Damage` (* (+ (`local.StatValuePercent`) 1.0) (`self.Damage`)))
    (elif (== StatType "WFireRate")
      (set `self.FireRate` (* (+ (`local.StatValuePercent`) 1.0) (`self.FireRate`)))
      (elif (== StatType "WReloadSpeed")
        (set `self.ReloadSpeed` (* (- 1.0 (`local.StatValuePercent`)) (`self.ReloadSpeed`)))
        (else
          (return false)))))
  (return true))

(fn `UserConstructionScript`)