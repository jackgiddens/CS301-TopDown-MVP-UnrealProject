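; Rocket projectile actor that explodes when its mesh begins overlapping its Enemy actor, then destroys itself.
; The hit spawns an explosion emitter and applies full radial damage in a small radius, ignoring the player.
; Damage scales RocketDamage by the player's Damage stat from TempPlayerStats, with a random CritChance roll adding the CritDamage multiplier.
; An older single-target fire-damage call remains disconnected.
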(event `self.StaticMesh.OnComponentBeginOverlap`
  (params (OverlappedComponent :type "PrimitiveComponent Object Reference") (OtherActor :type "Actor Object Reference") (OtherComp :type "PrimitiveComponent Object Reference") (OtherBodyIndex :type Integer) (bFromSweep :type Boolean) (SweepResult :type "HitResult Structure (by ref)"))
  ;[1 1 1] If rocket hits enemy deal damage
  (if (== OtherActor (`self.Enemy`))
    (`GameplayStatics.SpawnEmitterAtLocation` "/Game/StarterContent/Particles/P_Explosion.P_Explosion" (`self.K2_GetActorLocation` OtherActor) (struct) (0.5 0.5 0.5))
    (bind _asbp_base_character (cast `/Game/ThirdPerson/Blueprints/CharacterClasses/BP_BaseCharacter` (`GameplayStatics.GetPlayerCharacter` 0)))
    (bind _tempplayerstats (`/Game/ThirdPerson/Blueprints/CharacterClasses/BP_BaseCharacter.TempPlayerStats` _asbp_base_character))
    (bind _returnvalue (* (+ (* (`BlueprintMapLibrary.Map_Find` _tempplayerstats "Damage") 0.01) 1.0) (`self.RocketDamage`)))
    (`GameplayStatics.ApplyRadialDamage` (`KismetMathLibrary.SelectFloat` (* _returnvalue (+ (* (`BlueprintMapLibrary.Map_Find` _tempplayerstats "CritDamage") 0.01) 1.0)) _returnvalue (<= (`KismetMathLibrary.RandomFloatInRange` 0.0 1.0) (* (`BlueprintMapLibrary.Map_Find` _tempplayerstats "CritChance") 0.01))) (`self.K2_GetActorLocation`) 75.0 null (`|MakeArray` (`GameplayStatics.GetPlayerCharacter` 0)) null null true)
    (`self.K2_DestroyActor`)))

(fn `UserConstructionScript`)