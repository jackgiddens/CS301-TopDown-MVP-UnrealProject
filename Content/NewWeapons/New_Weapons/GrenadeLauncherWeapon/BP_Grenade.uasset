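; BP_Grenade is a grenade projectile that explodes half a second after hitting something.
; On hit it turns on physics and gravity, then after the delay spawns an explosion emitter scaled to the damage radius.
; It applies full fire radial damage that ignores the player, scaled by the player character's temporary damage stat with a random critical-hit roll, then destroys itself.
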(event `self.Grenade.OnComponentHit`
  (params (HitComponent :type "PrimitiveComponent Object Reference") (OtherActor :type "Actor Object Reference") (OtherComp :type "PrimitiveComponent Object Reference") (NormalImpulse :type "Vector Structure") (Hit :type "HitResult Structure (by ref)"))
  (bind _grenade (`self.Grenade`))
  ;[1 1 1] Deal damage in radius 0.5 seconds after hitting an object
  (`PrimitiveComponent.SetSimulatePhysics` _grenade true)
  (`PrimitiveComponent.SetEnableGravity` _grenade true)
  (`KismetSystemLibrary.Delay` 0.5)
  (`GameplayStatics.SpawnEmitterAtLocation` "/Game/StarterContent/Particles/P_Explosion.P_Explosion" (`self.K2_GetActorLocation`) (struct) (`KismetMathLibrary.Conv_DoubleToVector` (/ (`self.DamageRadius`) 70.0)))
  (bind _asbp_base_character (cast `/Game/ThirdPerson/Blueprints/CharacterClasses/BP_BaseCharacter` (`GameplayStatics.GetPlayerCharacter` 0)))
  (bind _tempplayerstats (`/Game/ThirdPerson/Blueprints/CharacterClasses/BP_BaseCharacter.TempPlayerStats` _asbp_base_character))
  (bind _returnvalue (* (+ (* (`BlueprintMapLibrary.Map_Find` _tempplayerstats "Damage") 0.01) 1.0) (`self.Damage`)))
  (`GameplayStatics.ApplyRadialDamage` (`KismetMathLibrary.SelectFloat` (* _returnvalue (+ (* (`BlueprintMapLibrary.Map_Find` _tempplayerstats "CritDamage") 0.01) 1.0)) _returnvalue (<= (`KismetMathLibrary.RandomFloatInRange` 0.0 1.0) (* (`BlueprintMapLibrary.Map_Find` _tempplayerstats "CritChance") 0.01))) (`self.K2_GetActorLocation`) (`self.DamageRadius`) "/Game/DamageTypes/DamageType_Fire.DamageType_Fire_C" (`|MakeArray` (`GameplayStatics.GetPlayerCharacter` 0) :!type "Actor Object Reference") null null true)
  (`self.K2_DestroyActor`))

(fn `UserConstructionScript`)