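; BP_Boomerang is a weapon projectile that flies one spinning loop out from the player and back, then destroys itself.
; A timeline drives the orbit angle and yaw flips, while Tick pins StartPoint to the player and places the boomerang on an offset circle.
; Box overlaps with actors that cast to BP_BaseWeapons apply bludgeoning damage, scaled by the player's Damage stat with a CritChance roll for CritDamage.
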(event `self.ReceiveBeginPlay`
  ;[1 1 1] Lerp current angle and flip overtime for boomerang
  (bind (_direction _newtrack_0) (`Timeline|Timeline`)
    (:`Update`
      (set `self.CurrentAngle` (`KismetMathLibrary.Lerp` 0.0 6.28 _newtrack_0))
      (set `self.Flip` (`KismetMathLibrary.Lerp` 0.0 (* 360.0 5.0) _newtrack_0)))
    (:`Finished`
      (`self.K2_DestroyActor`))))

(event `self.ReceiveTick`
  (params (DeltaSeconds :type "Float (single-precision)"))
  (bind _radius (`self.Radius`))
  ;[1 1 1] Sets boomerang location in a circular motion
  (`SceneComponent.K2_SetWorldLocation` (`self.StartPoint`) (`self.K2_GetActorLocation` (`GameplayStatics.GetPlayerCharacter` 0)) false false)
  (`SceneComponent.K2_SetRelativeLocationAndRotation` (`self.Boomerang`) (`KismetMathLibrary.MakeVector` (+ (* (`KismetMathLibrary.Cos` (`self.CurrentAngle`)) _radius -1.0) _radius) (* (`KismetMathLibrary.Sin` (`self.CurrentAngle`)) (`self.Radius`) -1.0)) (`KismetMathLibrary.MakeRotator` 0.0 0.0 (`self.Flip`)) false false))

(event `self.Box.OnComponentBeginOverlap`
  (params (OverlappedComponent :type "PrimitiveComponent Object Reference") (OtherActor :type "Actor Object Reference") (OtherComp :type "PrimitiveComponent Object Reference") (OtherBodyIndex :type Integer) (bFromSweep :type Boolean) (SweepResult :type "HitResult Structure (by ref)"))
  ;[1 1 1] When boomerang overlaps with enemy deal damage
  (cast `/Game/NewWeapons/Bases/BP_BaseWeapons` OtherActor)
  (bind _asbp_third_person_character (cast `/Game/ThirdPerson/Blueprints/CharacterClasses/BP_BaseCharacter` (`GameplayStatics.GetPlayerCharacter` 0)))
  (bind _tempplayerstats (`/Game/ThirdPerson/Blueprints/CharacterClasses/BP_BaseCharacter.TempPlayerStats` _asbp_third_person_character))
  (bind _returnvalue (* (+ (* (`BlueprintMapLibrary.Map_Find` _tempplayerstats "Damage") 0.01) 1.0) (`self.Damage`)))
  (`GameplayStatics.ApplyDamage` OtherActor (`KismetMathLibrary.SelectFloat` (* _returnvalue (+ (* (`BlueprintMapLibrary.Map_Find` _tempplayerstats "CritDamage") 0.01) 1.0)) _returnvalue (<= (`KismetMathLibrary.RandomFloatInRange` 0.0 1.0) (* (`BlueprintMapLibrary.Map_Find` _tempplayerstats "CritChance") 0.01))) null null "/Game/DamageTypes/DamageType_Bludgeoning.DamageType_Bludgeoning_C"))

(fn `UserConstructionScript`)