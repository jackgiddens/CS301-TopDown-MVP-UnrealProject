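; Sniper bullet actor that deals piercing-type damage to enemies its static mesh overlaps.
; On overlap with a BP_BaseEnemies, it scales its base Damage by the player's Damage percentage from TempPlayerStats.
; A random roll against CritChance decides whether the CritDamage multiplier also applies.
; It destroys itself one second after applying damage rather than on impact, so further overlaps can still deal damage during that delay.
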(event `self.StaticMesh.OnComponentBeginOverlap`
  (params (OverlappedComponent :type "PrimitiveComponent Object Reference") (OtherActor :type "Actor Object Reference") (OtherComp :type "PrimitiveComponent Object Reference") (OtherBodyIndex :type Integer) (bFromSweep :type Boolean) (SweepResult :type "HitResult Structure (by ref)"))
  ;[1 1 1] If bullet overlaps with enemy deal damage
  (cast `/Game/Enemies/BP_BaseEnemies` OtherActor)
  (bind _asbp_base_character (cast `/Game/ThirdPerson/Blueprints/CharacterClasses/BP_BaseCharacter` (`GameplayStatics.GetPlayerCharacter` 0)))
  (bind _tempplayerstats (`/Game/ThirdPerson/Blueprints/CharacterClasses/BP_BaseCharacter.TempPlayerStats` _asbp_base_character))
  (bind _returnvalue (* (+ (* (`BlueprintMapLibrary.Map_Find` _tempplayerstats "Damage") 0.01) 1.0) (`self.Damage`)))
  (`GameplayStatics.ApplyDamage` OtherActor (`KismetMathLibrary.SelectFloat` (* _returnvalue (+ (* (`BlueprintMapLibrary.Map_Find` _tempplayerstats "CritDamage") 0.01) 1.0)) _returnvalue (<= (`KismetMathLibrary.RandomFloatInRange` 0.0 1.0) (* (`BlueprintMapLibrary.Map_Find` _tempplayerstats "CritChance") 0.01))) null null "/Game/DamageTypes/DamageType_Piercing.DamageType_Piercing_C")
  (`KismetSystemLibrary.Delay` 1.0)
  (`self.K2_DestroyActor`))

(fn `UserConstructionScript`)