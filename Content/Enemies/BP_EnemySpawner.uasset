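; BP_EnemySpawner is an actor that spawns queued enemy classes one at a time at its location.
; A looping timer started on BeginPlay calls SpawnEnemy, which spawns the front class as an AI pawn facing the Arrow, ignoring collision, then removes it.
; AddEnemyToQueue appends classes to the queue.
; A Box overlap check against BP_BaseEnemies exists but is disconnected, so occupancy never blocks spawning.
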(event `self.ReceiveBeginPlay`
  (`KismetSystemLibrary.K2_SetTimerDelegate` (delegate `TryToSpawn`) 3.0 true))

(event `TryToSpawn`
  (`self.SpawnEnemy`))

(fn `AddEnemyToQueue`
  (params (EnemyClass :type "Pawn Class Reference (by ref)"))
  (`KismetArrayLibrary.Array_Add` (`self.EnemyQueue`) EnemyClass))

(fn `SpawnEnemy`
  (returns (Success :type Boolean))
  (if (`KismetArrayLibrary.Array_IsValidIndex` (`self.EnemyQueue`))
    (`AIBlueprintHelperLibrary.SpawnAIFromClass` (`|GetArrayItem` (`self.EnemyQueue`)) null (`self.K2_GetActorLocation`) (`SceneComponent.K2_GetComponentRotation` (`self.Arrow`)) true null)
    (`KismetArrayLibrary.Array_Remove` (`self.EnemyQueue`))
    (return true)
    (else
      (return false))))

(fn `UserConstructionScript`)