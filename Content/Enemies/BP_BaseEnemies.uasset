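; Base enemy character for a wave-based game that loads data-table stats, scales health and damage by wave, and chases the player.
; It crawls forward on spawn via a timeline, then loops AI MoveTo, relocating when stuck.
; Capsule overlap drives timed damage to the player; incoming damage spawns damage displays, and death drops XP and sometimes medkits.
; Repeated move failures or excessive player distance destroy it and queue its class with the GameMode for respawn.
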(event `CrawlForward`
  (bind _returnvalue (`self.K2_GetActorLocation`))
  (set `self.DefaultMaxSpeed` (`self.MaxWalkSpeed`))
  (set `self.MaxWalkSpeed` 20.0)
  (set `PrimitiveComponent.bGenerateOverlapEvents` false (`self.Capsule`))
  (set `self.SpawnLocation` _returnvalue)
  (set `self.CrawlLocation` (+ _returnvalue (* (`KismetMathLibrary.GetForwardVector` (`self.K2_GetActorRotation`)) 100.0)))
  (bind (_direction _newtrack_0) (`Timeline|Timeline` :!via `PlayFromStart`)
    (:`Update`
      (`self.K2_SetActorLocation` (`KismetMathLibrary.VLerp` (`self.SpawnLocation`) (`self.CrawlLocation`) _newtrack_0)))
    (:`Finished`
      (`PrimitiveComponent.SetCollisionResponseToChannel` (`self.CapsuleComponent`) "ECC_WorldStatic" "ECR_Block")
      (set `CharacterMovementComponent.GravityScale` 1.0 (`self.CharacterMovement`))
      (set `self.MaxWalkSpeed` (`self.DefaultMaxSpeed`))
      (set `PrimitiveComponent.bGenerateOverlapEvents` true (`self.Capsule`))
      (`self.AIMove`)
      (`self.StartRunAnim`))))

(event `CheckDistTimer`
  (`KismetSystemLibrary.K2_SetTimerDelegate` (delegate `CheckDist`) 5.0 true))

(event `CheckDist`
  (if (> (`KismetMathLibrary.VSize` (- (`self.K2_GetActorLocation` (`GameplayStatics.GetPlayerCharacter` 0)) (`self.K2_GetActorLocation`))) 2000.0)
    (`self.Respawn`)))

(event `Respawn`
  (`KismetArrayLibrary.Array_Add` (`/Game/ThirdPerson/Blueprints/BP_ThirdPersonGameMode.EnemysToRespawn` (`self.GamemodeREF`)) (`GameplayStatics.GetObjectClass` self))
  (`self.K2_DestroyActor`)
  (`KismetSystemLibrary.PrintString` "Respawn"))

(event `self.ReceiveBeginPlay`
  (bind (_returnvalue_x _returnvalue_y) (`KismetMathLibrary.BreakVector` (`self.K2_GetActorLocation`)))
  ;[1 1 1] Set Character and Gamemode Reference, scale Strength and move AI
  (`self.Set Stats` "None")
  (bind _asbp_base_character (cast `/Game/ThirdPerson/Blueprints/CharacterClasses/BP_BaseCharacter` (`GameplayStatics.GetPlayerCharacter` 0)))
  (set `self.CharREF` _asbp_base_character)
  (bind _asbp_third_person_game_mode (cast `/Game/ThirdPerson/Blueprints/BP_ThirdPersonGameMode` (`GameplayStatics.GetGameMode`)))
  (set `self.GamemodeREF` _asbp_third_person_game_mode)
  (`self.ScaleStrength` (`/Game/ThirdPerson/Blueprints/BP_ThirdPersonGameMode.WaveNum` _asbp_third_person_game_mode))
  (`KismetSystemLibrary.Delay` 0.2)
  (`self.K2_SetActorLocation` (`KismetMathLibrary.MakeVector` _returnvalue_x _returnvalue_y 55.0))
  (`self.CrawlForward`))

(event `AIMove`
  ;[1 1 1] Move AI to Player
  (`|AIMoveTo` self (0.0 0.0 0.0) (`self.CharREF`)
    (:`OnSuccess`
      (`self.AIMove`))
    (:`OnFail`
      ;;[1 1 1] If AI repeatedly cant move Destroy Actor
      (`self.TryRelocateActor`)
      (bind _result (`/Engine/EditorBlueprintResources/StandardMacros.IncrementInt` (`self.AIFails`))
        (:`  `
          (bind _output_get (set `self.AIFails` _result))
          (if (>= _output_get 3)
            (`self.Respawn`)
            (else
              (`KismetSystemLibrary.Delay` 0.2)
              (`self.AIMove`))))))))

(event `TryRelocateActor`
  ;[1 1 1] Try to move actor if stuck
  (bind _randomlocation (`NavigationSystemV1.K2_GetRandomLocationInNavigableRadius` (`self.K2_GetActorLocation`) 100.0 null null))
  (`self.K2_SetActorLocation` _randomlocation))

(event `self.ReceiveAnyDamage`
  (params (Damage :type "Float (single-precision)") (DamageType :type "DamageType Object Reference") (InstigatedBy :type "Controller Object Reference") (DamageCauser :type "Actor Object Reference"))
  ;[1 1 1] Apply Damage
  (bind _damagetype (message `/Game/Interfaces/GetDamageType.GetDamageType` DamageType))
  (bind _returnvalue (`self.CalculateCurrentHealth` Damage _damagetype (`self.DamageTable`)))
  (`|SpawnActorFromClass` "/Game/UI/InGame/BP_DamageAmt.BP_DamageAmt_C" (`self.GetTransform`) "Undefined" "MultiplyWithRoot" null _returnvalue null)
  ;;[1 1 1] If Health = 0 Die
  (if (== (`self.CurrentHealth`) 0.0)
    (`self.Die`)))

(event `Die`
  ;[1 1 1] Destroy self, spawn Xp and maybe Health Pack
  (`self.K2_DestroyActor`)
  (bind _randomlocation (`NavigationSystemV1.K2_GetRandomLocationInNavigableRadius` (`self.K2_GetActorLocation`) 100.0 null null))
  (bind _newparam (`self.ReturnXpMaterial`))
  (`|SpawnActorFromClass` "/Game/Collectibles/New_Xp.New_Xp_C" (`KismetMathLibrary.MakeTransform` (`KismetMathLibrary.MakeVector` (.x _randomlocation) (.y _randomlocation) (+ (.z _randomlocation) 100.0))) "Undefined" "MultiplyWithRoot" null _newparam (`KismetMathLibrary.RandomIntegerInRange` (`self.MinXp`) (`self.MaxXp`)) null)
  (`/Game/ThirdPerson/Blueprints/BP_ThirdPersonGameMode.OnEnemyKilled` (`self.GamemodeREF`))
  (if (< (`KismetMathLibrary.RandomFloatInRange` 0.0 1.0) (`self.HealthDropChance`))
    (bind _randomlocation_2 (`NavigationSystemV1.K2_GetRandomLocationInNavigableRadius` (`self.K2_GetActorLocation`) 100.0 null null))
    (`|SpawnActorFromClass` "/Game/Collectibles/New_MedKit.New_MedKit_C" (`KismetMathLibrary.MakeTransform` (`KismetMathLibrary.MakeVector` (.x _randomlocation_2) (.y _randomlocation_2) (+ (.z _randomlocation_2) 100.0))) "Undefined" "MultiplyWithRoot" null 0 null)))

(event `self.Capsule.OnComponentBeginOverlap`
  (params (OverlappedComponent :type "PrimitiveComponent Object Reference") (OtherActor :type "Actor Object Reference") (OtherComp :type "PrimitiveComponent Object Reference") (OtherBodyIndex :type Integer) (bFromSweep :type Boolean) (SweepResult :type "HitResult Structure (by ref)"))
  ;[1 1 1] While overlapping with Player Character start dealing damage over time (DOT)
  (if (== OtherActor (`self.CharREF`))
    (set `self.IsOverlapping` true)
    (if (not (`self.IsAttacking`))
      (`self.StartDOT`)
      (`self.ApplyDamage`))))

(event `self.Capsule.OnComponentEndOverlap`
  (params (OverlappedComponent :type "PrimitiveComponent Object Reference") (OtherActor :type "Actor Object Reference") (OtherComp :type "PrimitiveComponent Object Reference") (OtherBodyIndex :type Integer))
  ;[1 1 1] While overlapping with Player Character start dealing damage over time (DOT)
  (if (== (`self.CharREF`) OtherActor)
    (set `self.IsOverlapping` false)))

(event `StartDOT`
  ;[1 1 1] Apply damage over time to Player Character
  (bind _returnvalue (`KismetSystemLibrary.K2_SetTimerDelegate` (delegate `ApplyDamage`) (`self.DamageTickSpeed`) true))
  (set `self.DOTTimer` _returnvalue))

(event `ApplyDamage`
  ;[1 1 1] Apply damage over time to Player Character
  (set `self.IsAttacking` true)
  (`GameplayStatics.ApplyDamage` (`self.CharREF`) (`self.Damage`))
  (`KismetSystemLibrary.Delay` (`self.DamageTickSpeed`))
  (set `self.IsAttacking` false)
  (if (not (`self.IsOverlapping`))
    (`KismetSystemLibrary.K2_ClearAndInvalidateTimerHandle` (`self.DOTTimer`))))

(fn `GetEnemyHealth`
  (returns (ReturnValue :type "Float (single-precision)"))
  (return (`self.MaxHealth`)))

(fn `GetHealth`
  (returns (MaxHealth :type "Float (double-precision)"))
  (return 0.0))

(fn `ReturnXpMaterial`
  (returns (NewParam :type "Material Object Reference"))
  (return null))

(fn `ScaleStrength`
  (params (Wave :type Integer))
  (locals (MaxHealthMultiplier :type "Float (double-precision)" :default 0.06) (DamageMultiplier :type "Float (double-precision)" :default 0.05))
  (bind _output_get (set `self.MaxHealth` (* (+ (* (`KismetMathLibrary.Conv_IntToDouble` Wave) (`local.MaxHealthMultiplier`)) 1.0) (`self.MaxHealth`))))
  (set `self.CurrentHealth` _output_get)
  (set `self.Damage` (* (+ (* (`KismetMathLibrary.Conv_IntToDouble` (`local.Wave`)) (`local.DamageMultiplier`)) 1.0) (`self.Damage`))))

(fn `Set Stats`
  (params (RowName :type Name))
  (bind _returnvalue (`|GetDataTableRow` "/Game/Data/DataTables/EnemiesDataTable.EnemiesDataTable" RowName)
    (:`then`
      (bind (_name _spawnchance _damage _damagetickspeed _damagetable _maxhealth _maxwalkspeed _minxp _maxhp _healthdropchance) (break `/Game/Data/Sturctures/EnemiesStruct` _returnvalue))
      (set `self.Damage` _damage)
      (set `self.DamageTickSpeed` _damagetickspeed)
      (set `self.DamageTable` _damagetable)
      (set `self.MaxHealth` _maxhealth)
      (set `self.MaxWalkSpeed` _maxwalkspeed)
      (set `self.MinXp` _minxp)
      (set `self.MaxXp` _maxhp)
      (set `self.HealthDropChance` _healthdropchance)
      (set `CharacterMovementComponent.MaxWalkSpeed` (`self.MaxWalkSpeed`) (`self.CharacterMovement`)))))

(fn `UserConstructionScript`)