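; Base enemy spawner in the car spawners folder that registers with the third-person game mode while the player is in range.
; A sphere's overlaps add or remove it from the game mode's Spawners array, with a delayed BeginPlay check for a player already inside.
; SpawnEnemy spawns a given AI class at the actor's location, facing along an arrow whose yaw FlipSpawn negates at start.
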(event `self.ReceiveBeginPlay`
  (bind _arrow (`self.Arrow`))
  (bind (_relativerotation_roll _relativerotation_pitch _relativerotation_yaw) (`KismetMathLibrary.BreakRotator` (`SceneComponent.RelativeRotation` _arrow)))
  ;[1 1 1] Set gamemode reference, add spawners within range to array and check flip spawner
  (`KismetSystemLibrary.Delay` 0.2)
  (bind _asbp_third_person_game_mode (cast `/Game/ThirdPerson/Blueprints/BP_ThirdPersonGameMode` (`GameplayStatics.GetGameMode`)))
  (set `self.GameModeREF` _asbp_third_person_game_mode)
  (`self.AddSpawners`)
  (if (`self.FlipSpawn`)
    (`SceneComponent.K2_SetRelativeRotation` _arrow (`KismetMathLibrary.MakeRotator` _relativerotation_roll _relativerotation_pitch (* _relativerotation_yaw -1.0)) false false)))

(event `AddSpawners`
  ;[1 1 1] Add spawners within range to array on begin play
  (if (`PrimitiveComponent.IsOverlappingActor` (`self.Sphere`) (`GameplayStatics.GetPlayerCharacter` 0))
    (`KismetArrayLibrary.Array_Add` (`/Game/ThirdPerson/Blueprints/BP_ThirdPersonGameMode.Spawners` (`self.GameModeREF`)) self)))

(event `self.Sphere.OnComponentBeginOverlap`
  (params (OverlappedComponent :type "PrimitiveComponent Object Reference") (OtherActor :type "Actor Object Reference") (OtherComp :type "PrimitiveComponent Object Reference") (OtherBodyIndex :type Integer) (bFromSweep :type Boolean) (SweepResult :type "HitResult Structure (by ref)"))
  ;[1 1 1] Keeps track of spawners within player range
  (cast `/Game/ThirdPerson/Blueprints/CharacterClasses/BP_BaseCharacter` OtherActor)
  (`KismetArrayLibrary.Array_Add` (`/Game/ThirdPerson/Blueprints/BP_ThirdPersonGameMode.Spawners` (`self.GameModeREF`)) self))

(event `self.Sphere.OnComponentEndOverlap`
  (params (OverlappedComponent :type "PrimitiveComponent Object Reference") (OtherActor :type "Actor Object Reference") (OtherComp :type "PrimitiveComponent Object Reference") (OtherBodyIndex :type Integer))
  ;[1 1 1] Keeps track of spawners within player range
  (cast `/Game/ThirdPerson/Blueprints/CharacterClasses/BP_BaseCharacter` OtherActor)
  (`KismetArrayLibrary.Array_RemoveItem` (`/Game/ThirdPerson/Blueprints/BP_ThirdPersonGameMode.Spawners` (`self.GameModeREF`)) self))

(fn `SpawnEnemy`
  (params (EnemyClass :type "Pawn Class Reference"))
  ;[1 1 1] Spawns enemy at spawner location
  (`AIBlueprintHelperLibrary.SpawnAIFromClass` EnemyClass null (`self.K2_GetActorLocation`) (`SceneComponent.K2_GetComponentRotation` (`self.Arrow`)) true null))

(fn `UserConstructionScript`)