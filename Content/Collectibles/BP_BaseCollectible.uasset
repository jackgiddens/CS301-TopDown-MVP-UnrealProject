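; Base collectible actor that is pulled toward the player character and can despawn after a set duration.
; Overlapping the Magnet component plays a timeline that lerps the actor from its current location to the player's live position.
; Once StartDespawnTimer is called, a one-second looping timer counts elapsed time, blinks the mesh as expiry nears, speeds up the blink shortly before the end, then destroys the actor.
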(event `self.ReceiveBeginPlay`
  ;[1 1 1] Set Player Character reference
  (bind _asbp_base_character (cast `/Game/ThirdPerson/Blueprints/CharacterClasses/BP_BaseCharacter` (`GameplayStatics.GetPlayerCharacter` 0)))
  (set `self.PlayerCharREF` _asbp_base_character))

(event `self.Magnet.OnComponentBeginOverlap`
  (params (OverlappedComponent :type "PrimitiveComponent Object Reference") (OtherActor :type "Actor Object Reference") (OtherComp :type "PrimitiveComponent Object Reference") (OtherBodyIndex :type Integer) (bFromSweep :type Boolean) (SweepResult :type "HitResult Structure (by ref)"))
  ;[1 1 1] Move towards the Player Character when they are within magnet range
  (if (== OtherActor (`self.PlayerCharREF`))
    (bind (_direction _moveactor) (`Timeline|MoveToPlayer` :!via `PlayFromStart`)
      (:`Update`
        (`self.K2_SetActorLocation` (`KismetMathLibrary.VLerp` (`self.K2_GetActorLocation`) (`self.K2_GetActorLocation` (`self.PlayerCharREF`)) _moveactor))))))

(event `StartDespawnTimer`
  (`KismetSystemLibrary.K2_SetTimerDelegate` (delegate `DespawnTimer`) 1.0 true))

(event `DespawnTimer`
  (bind _despawnduration (`self.DespawnDuration`))
  (bind _result (`/Engine/EditorBlueprintResources/StandardMacros.IncrementFloat` (`self.ElapsedTime`))
    (:`  `
      (if (== _result (- _despawnduration 6.0))
        (`self.StartDespawnWarning` :!label _label)
        (elif (== (`self.ElapsedTime`) (- _despawnduration 2.0))
          (`KismetSystemLibrary.K2_ClearAndInvalidateTimerHandle` (`self.DespawnWarningTimer`))
          (set `self.WarningFlashTime` 0.15)
          (goto _label)
          (elif (>= (`self.ElapsedTime`) (`self.DespawnDuration`))
            (`self.K2_DestroyActor`)))))))

(event `StartDespawnWarning`
  (bind _returnvalue (`KismetSystemLibrary.K2_SetTimerDelegate` (delegate `DespawnWarning`) (`self.WarningFlashTime`) true))
  (set `self.DespawnWarningTimer` _returnvalue))

(event `DespawnWarning`
  (if (`self.Hidden`)
    (set `self.Hidden` false)
    (else
      (set `self.Hidden` true)))
  (`SceneComponent.SetHiddenInGame` (`self.StaticMesh`) (`self.Hidden`) false))

(fn `UserConstructionScript`)